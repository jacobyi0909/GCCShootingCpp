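; BP_CodingActor is a test actor that exercises Blueprint-callable, pure and overridable event functions, apparently from a parent class.
; On BeginPlay it prints the result of AddPure; the AddCallable call and the prints of Num, Speed, Good and MyName are disconnected.
; AddImplEvent implements its own addition, while AddNativeEvent calls the parent version, then prints and returns that result.
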(event EventBeginPlay
  (Development|PrintString (Utilities|String|ToString(Integer) (Class|CodingActor|AddPure 100 200)) true true "(R=0.000000,G=0.660000,B=1.000000,A=1.000000)" 5e+01))

(event Collision|EventActorBeginOverlap
  (params (OtherActor :type Actor%20Object%20Reference)))

(event EventTick
  (params (DeltaSeconds :type Float%20%28single-precision%29)))

(fn ConstructionScript)

(fn AddImplEvent
  (params (a :type Integer) (b :type Integer))
  (return (+ a b)))

(fn AddNativeEvent
  (params (a :type Integer) (b :type Integer))
  (bind _returnvalue (|CallParentFunction a b))
  (Development|PrintString (Utilities|String|ToString(Integer) _returnvalue))
  (return _returnvalue))